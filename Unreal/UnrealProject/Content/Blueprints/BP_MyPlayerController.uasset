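; Player controller that turns look and movement axis inputs into actions on the controlled pawn.
; Mouse look axes feed yaw and pitch directly, while stick look axes are scaled by RotationSpeed and frame delta time for frame-rate-independent turning.
; Forward and right movement axes add movement input along the pawn's own forward and right vectors.
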(event `InputAxis|LookAtRightMouse`
  (params (AxisValue :type "Float (single-precision)"))
  ;[1 1 1] Mouse Control
  (`Pawn.AddControllerYawInput` (`self.K2_GetPawn`) AxisValue))

(event `InputAxis|LookAtUpMouse`
  (params (AxisValue :type "Float (single-precision)"))
  ;[1 1 1] Mouse Control
  (`Pawn.AddControllerPitchInput` (`self.K2_GetPawn`) AxisValue))

(event `InputAxis|LookAtRight`
  (params (AxisValue :type "Float (single-precision)"))
  ;[1 1 1] Stick Control
  (`Pawn.AddControllerYawInput` (`self.K2_GetPawn`) (* AxisValue (`self.RotationSpeed`) (`GameplayStatics.GetWorldDeltaSeconds`))))

(event `InputAxis|LookAtUp`
  (params (AxisValue :type "Float (single-precision)"))
  ;[1 1 1] Stick Control
  (`Pawn.AddControllerPitchInput` (`self.K2_GetPawn`) (* AxisValue (`self.RotationSpeed`) (`GameplayStatics.GetWorldDeltaSeconds`))))

(event `InputAxis|MovementForward`
  (params (AxisValue :type "Float (single-precision)"))
  (bind _returnvalue (`self.K2_GetPawn`))
  ;[1 1 1] Movement control
  (`Pawn.AddMovementInput` _returnvalue (`self.GetActorForwardVector` _returnvalue) AxisValue false))

(event `InputAxis|MovementRight`
  (params (AxisValue :type "Float (single-precision)"))
  (bind _returnvalue (`self.K2_GetPawn`))
  ;[1 1 1] Movement control
  (`Pawn.AddMovementInput` _returnvalue (`self.GetActorRightVector` _returnvalue) AxisValue false))

(fn `UserConstructionScript`)