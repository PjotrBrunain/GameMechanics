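; BP_LockPick is a lockpick Blueprint that shows and hides one of two widgets depending on whether it is disabled.
; On BeginPlay it moves both the normal and disabled widgets to a shared configurable relative location.
; ShowWidget reveals the widget matching the Disabled flag, and HideWidget hides both.
; No lockpicking logic lives in its graphs.
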(event `self.ReceiveBeginPlay`
  (`SceneComponent.K2_SetRelativeLocation` (`self.Widget`) (`self.WidgetLocation`) false false)
  (`SceneComponent.K2_SetRelativeLocation` (`self.WidgetDisabled`) (`self.WidgetLocation`) false false))

(event `/Game/Blueprints/InteractInterface.ShowWidget`
  (if (`self.Disabled`)
    (`SceneComponent.SetVisibility` (`self.WidgetDisabled`) true false)
    (else
      (`SceneComponent.SetVisibility` (`self.Widget`) true false))))

(event `/Game/Blueprints/InteractInterface.HideWidget`
  (`SceneComponent.SetVisibility` (`self.WidgetDisabled`) false false)
  (`SceneComponent.SetVisibility` (`self.Widget`) false false))

(fn `UserConstructionScript`)