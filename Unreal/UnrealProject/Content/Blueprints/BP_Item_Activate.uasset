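; BP_Item_Activate is an activatable item that toggles between active and inactive and can be disabled.
; Activate flips IsActive and calls the Activated dispatcher, but only while the item is not Disabled.
; Two widget components share WidgetLocation, set on BeginPlay; ShowWidget reveals the normal or disabled one based on Disabled, and HideWidget hides both.
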(event `Activate`
  (if (not (`self.Disabled`))
    (set `self.IsActive` (not (`self.IsActive`)))
    (`self.Activated`)))

(event `self.ReceiveBeginPlay`
  ;[1 1 1] Widget
  (`SceneComponent.K2_SetRelativeLocation` (`self.Widget`) (`self.WidgetLocation`) false false)
  (`SceneComponent.K2_SetRelativeLocation` (`self.WidgetDisabled`) (`self.WidgetLocation`) false false))

(event `/Game/Blueprints/InteractInterface.ShowWidget`
  ;[1 1 1] Widget
  (if (`self.Disabled`)
    (`SceneComponent.SetVisibility` (`self.WidgetDisabled`) true false)
    (else
      (`SceneComponent.SetVisibility` (`self.Widget`) true false))))

(event `/Game/Blueprints/InteractInterface.HideWidget`
  ;[1 1 1] Widget
  (`SceneComponent.SetVisibility` (`self.WidgetDisabled`) false false)
  (`SceneComponent.SetVisibility` (`self.Widget`) false false))

(fn `UserConstructionScript`)